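; Ladder prop ("escada") that lets MainChar climb while inside its trigger Box.
; The construction script stacks collision-free Paper2D sprites every Rungoffset units, counted from the Z difference between Escadabaixo and Escadatopo.
; It also scales and raises the Box using that same height.
; Overlap begin sets the character's CanClimb; overlap end clears it and calls SubiDescer on the character.
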(event OnComponentBeginOverlap(Box)
  (params (OverlappedComponent :type Primitive%20Component%20Object%20Reference) (OtherActor :type Actor%20Object%20Reference) (OtherComp :type Primitive%20Component%20Object%20Reference) (OtherBodyIndex :type Integer) (bFromSweep :type Boolean) (SweepResult :type Hit%20Result%20Structure%20%28by%20ref%29))
  (bind _asmain_char (Utilities|Casting|CastToMainChar OtherActor))
  (Variables|/Game/Game/BluePrint/MainChar.MainChar_C|SetbCanClimb _asmain_char true))

(event OnComponentEndOverlap(Box)
  (params (OverlappedComponent :type Primitive%20Component%20Object%20Reference) (OtherActor :type Actor%20Object%20Reference) (OtherComp :type Primitive%20Component%20Object%20Reference) (OtherBodyIndex :type Integer))
  (bind _asmain_char (Utilities|Casting|CastToMainChar OtherActor))
  (Variables|/Game/Game/BluePrint/MainChar.MainChar_C|SetbCanClimb _asmain_char false)
  (Default|SubiDescer _asmain_char))

(fn ConstructionScript
  (bind _box (Variables|Default|GetBox))
  (bind _escadatopo (Variables|Default|Getescadatopo))
  (bind _escadabaixo (Variables|Default|Getescadabaixo))
  (bind _rungoffset (Variables|Default|Getrungoffset))
  (bind _returnvalue (- _escadabaixo _escadatopo))
  (bind _returnvalue_2 (/ (.z _returnvalue) 2.0))
  ;[1 1 1] Comment
  (for _index (range 0 (Math|Float|Truncate (/ (.z _returnvalue) _rungoffset)))
    (bind _returnvalue_3 (AddComponent|AddPaperSpriteComponent false (Math|Transform|MakeTransform (Math|Vector|MakeVector 0.0 0.0 (* _index _rungoffset)) "0, 0, 0" "1,1,1")))
    (Rendering|Components|Sprite|SetSprite _returnvalue_3 (Variables|Default|Getescadasprite))
    (Collision|SetCollisionEnabled _returnvalue_3 "NoCollision"))
  (Transformation|SetRelativeScale3D _box (Math|Vector|MakeVector 2.0 2.0 _returnvalue_2))
  (Transformation|AddRelativeLocation _box (Math|Vector|MakeVector 0.0 0.0 _returnvalue_2) false false))